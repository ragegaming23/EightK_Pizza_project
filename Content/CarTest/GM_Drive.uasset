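; GM_Drive is the game mode for a driving game with delivery missions, handling car respawns and the win condition.
; RespawnPlayer plays an explosion sound, waits briefly, then spawns a new BP_Car2 at the given transform and possesses it.
; AddMission registers unique targets, and CountMission removes completed ones.
; When the list empties, it pauses the game after a short delay and shows WB_WinScreen with UI-only input.
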(event Custom|Respawn%20Player
  (params (SpawnTransform :type Transform))
  (Audio|PlaySound2D "/Game/StarterContent/Audio/Explosion01.Explosion01" 1.0 1.0 0.0 0 0)
  (Utilities|FlowControl|Delay 3.0)
  (bind _returnvalue (Game|SpawnActorfromClass "/Game/Car2/BP_Car2.BP_Car2_C" SpawnTransform "Undefined" "MultiplyWithRoot" 0 0))
  (Pawn|Possess (Game|GetPlayerController 0) _returnvalue))

(event EventAddMission
  (params (Mission :type BP%20Mission%20Object%20Reference))
  (Utilities|Array|AddUnique (Variables|Default|GetTargetMissions) Mission))

(event EventCountMission
  (params (Mission :type BP%20Mission%20Object%20Reference))
  (bind _returnvalue (Game|GetPlayerCharacter 0))
  (bind _playerstate (Variables|/Script/Engine.Pawn|GetPlayerState _returnvalue))
  (bind _returnvalue_2 (Game|GetPlayerController _playerstate))
  (bind _returnvalue_3 (Utilities|Array|RemoveItem (Variables|Default|GetTargetMissions) Mission))
  (if _returnvalue_3
    (Development|PrintString "Delivery Complete")
    (if (Utilities|Array|IsEmpty (Variables|Default|GetTargetMissions))
      (Utilities|FlowControl|Delay 0.4)
      (Game|SetGamePaused true)
      (bind _returnvalue_4 (UserInterface|CreateWidget "/Game/WinScreen/WB_WinScreen.WB_WinScreen_C"))
      (UserInterface|Viewport|AddtoViewport _returnvalue_4 0)
      (Input|SetInputModeUIOnly _returnvalue_2 0 "DoNotLock" false)
      (Variables|/Script/Engine.PlayerController|SetbShowMouseCursor _returnvalue_2 true))))

(fn ConstructionScript)