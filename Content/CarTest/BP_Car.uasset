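; Drivable car pawn for a delivery game, pushed by physics force up to a top speed and steered by fixed yaw steps through Enhanced Input.
; Tick scales engine audio pitch with speed and sphere-traces from camera to body, fading blocking buildings through a dynamic material "Mask" parameter.
; The shoot input toggles the HUD delivery widget, gating driving inputs while open and printing success on close if the meter is near centre.
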(event Input|EnhancedActionEvents|EnhancedInputActionEA_Forward
  (params (ActionValue :type Boolean) (ElapsedSeconds :type Float%20%28double-precision%29) (TriggeredSeconds :type Float%20%28double-precision%29) (InputAction :type Input%20Action%20Object%20Reference :default "/Game/CarTest/Input/EA_Forward.EA_Forward"))
  (Utilities|FlowControl|Gate false
    (:Exit
      (CallFunction|Accelerate (Math|Vector|GetForwardVector (Variables|Default|GetBody))))))

(event Input|EnhancedActionEvents|EnhancedInputActionEA_Right
  (params (ActionValue :type Boolean) (ElapsedSeconds :type Float%20%28double-precision%29) (TriggeredSeconds :type Float%20%28double-precision%29) (InputAction :type Input%20Action%20Object%20Reference :default "/Game/CarTest/Input/EA_Right.EA_Right"))
  (Utilities|FlowControl|Gate false
    (:Exit
      (Transformation|AddWorldRotation (Variables|Default|GetBody) "0.000000,1.500000,0.000000" false false))))

(event Input|EnhancedActionEvents|EnhancedInputActionEA_Left
  (params (ActionValue :type Boolean) (ElapsedSeconds :type Float%20%28double-precision%29) (TriggeredSeconds :type Float%20%28double-precision%29) (InputAction :type Input%20Action%20Object%20Reference :default "/Game/CarTest/Input/EA_Left.EA_Left"))
  (Utilities|FlowControl|Gate false
    (:Exit
      (Transformation|AddWorldRotation (Variables|Default|GetBody) "0.000000,-1.500000,0.000000" false false))))

(event Input|EnhancedActionEvents|EnhancedInputActionEA_Shoot
  (params (ActionValue :type Boolean) (ElapsedSeconds :type Float%20%28double-precision%29) (TriggeredSeconds :type Float%20%28double-precision%29) (InputAction :type Input%20Action%20Object%20Reference :default "/Game/CarTest/Input/EA_Shoot.EA_Shoot"))
  (bind _deliverrange (Variables|Default|GetDeliverRange))
  (bind _body (Variables|Default|GetBody))
  (bind _returnvalue (Actor|GetActorOfClass "/Game/CarTest/HUD_Delivery.HUD_Delivery_C"))
  (Utilities|FlowControl|FlipFlop
    (:A
      (UserInterface|Viewport|AddtoViewport (Variables|/Game/CarTest/HUD_Delivery.HUD_Delivery_C|GetDelivery%20Widget _returnvalue) 0)
      (Utilities|FlowControl|Sequence
        (:then_0
          (Utilities|FlowControl|Gate false) ; enters at Close
        )
        (:then_1
          (Utilities|FlowControl|Gate false) ; enters at Close
        )
        (:then_2
          (Utilities|FlowControl|Gate false) ; enters at Close
        )))
    (:B
      (Widget|RemovefromParent (Variables|/Game/CarTest/HUD_Delivery.HUD_Delivery_C|GetDelivery%20Widget _returnvalue))
      (if (and (>= (Variables|/Game/CarTest/HUD_Delivery.HUD_Delivery_C|GetMeter%20Value _returnvalue) (- 0.5 _deliverrange)) (<= (Variables|/Game/CarTest/HUD_Delivery.HUD_Delivery_C|GetMeter%20Value _returnvalue) (+ 0.5 _deliverrange)))
        (Development|PrintString "SUCCESS!"))
      (Utilities|FlowControl|Sequence
        (:then_0
          (Utilities|FlowControl|Gate false) ; enters at Open
        )
        (:then_1
          (Utilities|FlowControl|Gate false) ; enters at Open
        )
        (:then_2
          (Utilities|FlowControl|Gate false) ; enters at Open
        )))))

(event EventBeginPlay
  (bind _asplayer_controller (Utilities|Casting|CastToPlayerController (Pawn|GetController)))
  (Utilities|IsValid (PlayerController|LocalPlayerSubsystems|GetEnhancedInputLocalPlayerSubsystem _asplayer_controller)
    (:Is%20Valid
      (Input|AddMappingContext (PlayerController|LocalPlayerSubsystems|GetEnhancedInputLocalPlayerSubsystem _asplayer_controller) "/Game/CarTest/Input/Map_Drive.Map_Drive" 0 "(bIgnoreAllPressedKeysUntilRelease=True,bForceImmediately=False,bNotifyUserSettings=False)"))))

(event Collision|EventActorBeginOverlap
  (params (OtherActor :type Actor%20Object%20Reference)))

(event EventTick
  (params (DeltaSeconds :type Float%20%28single-precision%29))
  (bind _buildings (Variables|Default|GetBuildings))
  (Utilities|FlowControl|Sequence
    (:then_0
      (Variables|Default|SetCurrentSpeed (Math|Vector|VectorLength (Transformation|GetComponentVelocity (Variables|Default|GetBody))))
      (bind _outhit (Collision|SphereTraceByChannel (Transformation|GetWorldLocation (Variables|Default|GetCamera)) (Transformation|GetWorldLocation (Variables|Default|GetBody)) 3e+01 "TraceTypeQuery3" false 0 "None" false))
      (if (== (Variables|Default|GetBody) (.HitComponent (Collision|BreakHitResult _outhit)))
        (for _array_element _buildings
          (bind _returnvalue (Rendering|Material|CreateDynamicMaterialInstance _array_element 0 (Rendering|Material|GetMaterial _array_element 0) "None" :!class /Script/Engine.PrimitiveComponent))
          (Rendering|Material|SetScalarParameterValue _returnvalue "Mask" 1.0 :!class /Script/Engine.MaterialInstanceDynamic))
        (Utilities|Array|Clear _buildings)
        (else
          (Utilities|Array|Add (Variables|Default|GetBuildings) (.HitComponent (Collision|BreakHitResult _outhit)))
          (for _array_element_2 (Variables|Default|GetBuildings)
            (if (== _array_element_2 (.HitComponent (Collision|BreakHitResult _outhit)))
              (bind _returnvalue_2 (Rendering|Material|CreateDynamicMaterialInstance _array_element_2 0 (Rendering|Material|GetMaterial _array_element_2 0) "None" :!class /Script/Engine.PrimitiveComponent))
              (Rendering|Material|SetScalarParameterValue _returnvalue_2 "Mask" 0.25 :!class /Script/Engine.MaterialInstanceDynamic)
              (else
                (bind _returnvalue_3 (Rendering|Material|CreateDynamicMaterialInstance _array_element_2 0 (Rendering|Material|GetMaterial _array_element_2 0) "None" :!class /Script/Engine.PrimitiveComponent))
                (Rendering|Material|SetScalarParameterValue _returnvalue_3 "Mask" 1.0 :!class /Script/Engine.MaterialInstanceDynamic)
                (Utilities|Array|RemoveItem (Variables|Default|GetBuildings) _array_element_2)))))))
    (:then_1
      (Audio|Components|Audio|SetPitchMultiplier (Variables|Default|Getcivic_dyno_Idol_Loop_mixdown_Cue) (+ (/ (Variables|Default|GetCurrentSpeed) (Variables|Default|GetTopSpeed)) 0.5)))))

(fn ConstructionScript)

(fn Accelerate
  (params (Direction :type Vector))
  (if (< (Variables|Default|GetCurrentSpeed) (Variables|Default|GetTopSpeed))
    (Physics|AddForce (Variables|Default|GetBody) (* Direction (Variables|Default|GetAcceleration)) "None" true)))

(fn Rotate
  (bind _body (Variables|Default|GetBody))
  (bind _body_2 (Variables|Default|GetBody))
  (bind _returnvalue (Transformation|GetComponentVelocity _body))
  (bind _returnvalue_2 (Transformation|GetWorldRotation _body_2))
  (if (> (Math|Vector|VectorLengthXY _returnvalue) 1e+01)
    (Transformation|SetWorldRotation (Variables|Default|GetBody) (Math|Rotator|Lerp(Rotator) (Math|Rotator|MakeRotator (.roll _returnvalue_2) (.pitch _returnvalue_2) (.yaw _returnvalue_2)) (Math|Rotator|MakeRotator (.roll _returnvalue_2) (.pitch _returnvalue_2) (Class|KismetAnimationLibrary|CalculateDirection _returnvalue (Math|Rotator|MakeRotator 0.0 0.0 0.0))) 0.5) false false)))

(fn IsPlayer
  (return (Pawn|IsPlayerControlled)))