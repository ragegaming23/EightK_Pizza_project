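; BP_Explosive is an actor that explodes on a timer after the player touches it, as a visual effect with no damage logic.
; A capsule overlap uses an IsPlayerMessage call on the other actor to filter for the player.
; After a short delay it zeroes the mesh's physics velocity, hides it and attaches the NS_Explosion Niagara effect.
; A second delay lets the effect play before the actor destroys itself.
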(event OnComponentBeginOverlap(Capsule)
  (params (OverlappedComponent :type Primitive%20Component%20Object%20Reference) (OtherActor :type Actor%20Object%20Reference) (OtherComp :type Primitive%20Component%20Object%20Reference) (OtherBodyIndex :type Integer) (bFromSweep :type Boolean) (SweepResult :type Hit%20Result%20Structure%20%28by%20ref%29))
  (bind _isplayer (Class|BPIPlayer|IsPlayer(Message) OtherActor))
  (if _isplayer
    (Utilities|FlowControl|Delay 3.0)
    (Class|PrimitiveComponent|SetAllPhysicsLinearVelocity (Variables|Default|GetStaticMesh) "0, 0, 0" false)
    (Rendering|SetVisibility (Variables|Default|GetStaticMesh) false false)
    (Niagara|SpawnSystemAttached "/Game/CarTest/NS_Explosion.NS_Explosion" (Variables|Default|GetStaticMesh) "None" "0, 0, 0" "0, 0, 0" "KeepRelativeOffset" true)
    (Utilities|FlowControl|Delay 2.0)
    (Actor|DestroyActor)))

(event EventBeginPlay)

(event Collision|EventActorBeginOverlap
  (params (OtherActor :type Actor%20Object%20Reference)))

(event EventTick
  (params (DeltaSeconds :type Float%20%28single-precision%29)))

(fn ConstructionScript)