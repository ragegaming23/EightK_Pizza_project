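; TestCube is an actor that points an arrow toward the nearest delivery pin.
; GiveDeliveryPoint and RemoveDeliveryPoint maintain the pin list, with removal printing a debug string but leaving the cached nearest pin untouched.
; Each tick scans the list for the closest pin, then smoothly turns the arrow's yaw toward it using Atan2 and a shortest-path lerp with fixed alpha.
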(event EventBeginPlay)

(event Collision|EventActorBeginOverlap
  (params (OtherActor :type Actor%20Object%20Reference)))

(event EventTick
  (params (DeltaSeconds :type Float%20%28single-precision%29))
  (bind _defaultsceneroot (Variables|Default|GetDefaultSceneRoot))
  (bind _returnvalue (Transformation|GetWorldLocation _defaultsceneroot))
  (Utilities|FlowControl|Sequence
    (:then_0
      (for _array_element (Variables|Default|GetDeliveryPins)
        (if (or (not (Utilities|IsValid (Variables|Default|GetcurrentNearestPin))) (< (Math|Vector|Distance(Vector) (Transformation|GetWorldLocation (Variables|/Game/Blueprints/MissionPin.MissionPin_C|GetDefaultSceneRoot _array_element)) (Transformation|GetWorldLocation (Variables|Default|GetDefaultSceneRoot))) (Variables|Default|GetcurrentNearestDistance)))
          (Variables|Default|SetcurrentNearestPin _array_element)
          (Variables|Default|SetcurrentNearestDistance (Math|Vector|Distance(Vector) (Transformation|GetWorldLocation (Variables|/Game/Blueprints/MissionPin.MissionPin_C|GetDefaultSceneRoot _array_element)) (Transformation|GetWorldLocation (Variables|Default|GetDefaultSceneRoot))))
          (else
            (Variables|Default|SetcurrentNearestDistance (Transformation|GetDistanceTo (Variables|Default|GetcurrentNearestPin)))))))
    (:then_1
      (Utilities|IsValid (Variables|Default|GetcurrentNearestPin)
        (:Is%20Valid
          (Transformation|SetWorldRotation (Variables|Default|GetArrow) (Math|Rotator|Lerp(Rotator) (Math|Rotator|MakeRotator 0.0 0.0 (.yaw (Transformation|GetWorldRotation (Variables|Default|GetArrow)))) (Math|Rotator|MakeRotator 0.0 0.0 (+ (Class|KismetMathLibrary|DegAtan2 (- (.y _returnvalue) (.y (Transformation|GetWorldLocation (Variables|/Game/Blueprints/MissionPin.MissionPin_C|GetDefaultSceneRoot (Variables|Default|GetcurrentNearestPin))))) (- (.x _returnvalue) (.x (Transformation|GetWorldLocation (Variables|/Game/Blueprints/MissionPin.MissionPin_C|GetDefaultSceneRoot (Variables|Default|GetcurrentNearestPin)))))) 9e+01)) 0.25 true) false false))))))

(event EventGiveDeliveryPoint
  (params (Position :type Vector :default "0, 0, 0") (Pin :type Mission%20Pin%20Object%20Reference))
  (Utilities|Array|AddUnique (Variables|Default|GetDeliveryPins) Pin))

(event EventRemoveDeliveryPoint
  (params (Pin :type Mission%20Pin%20Object%20Reference))
  (Utilities|Array|RemoveItem (Variables|Default|GetDeliveryPins) Pin)
  (Development|PrintString "Hello"))

(fn ConstructionScript)