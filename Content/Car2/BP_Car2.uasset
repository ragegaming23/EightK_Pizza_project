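; Player-driven car that moves by physics forces along fixed world axes and fires BP_THEPIZZA projectiles from a cannon.
; A per-tick downward trace toggles movement gates and damping, adding extra downward force when airborne; grounded yaw eases toward the velocity direction.
; Speed drives engine and city-noise audio and spring arm length.
; Hard, fast hits on BPI_CollisionObject actors subtract the damage they return from Health.
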(event OnComponentHit(Body)
  (params (HitComponent :type Primitive%20Component%20Object%20Reference) (OtherActor :type Actor%20Object%20Reference) (OtherComp :type Primitive%20Component%20Object%20Reference) (NormalImpulse :type Vector :default "0, 0, 0") (Hit :type Hit%20Result%20Structure%20%28by%20ref%29))
  (if (Math|Boolean|ANDBoolean (Utilities|DoesObjectImplementInterface OtherActor "/Game/Blueprints/BPI_CollisionObject.BPI_CollisionObject_C") (> (Math|Vector2D|Vector2DLength (Math|Vector2D|MakeVector2D (.x NormalImpulse) (.y NormalImpulse))) 3.2e+04) (> (Variables|Default|GetCurrentSpeed) 6e+03))
    (bind _collisiondamage (Class|BPICollisionObject|Collidedwith(Message) OtherActor))
    (bind _output_get (Variables|Default|SetHealth (- (Variables|Default|GetHealth) _collisiondamage)))
    (Development|PrintString (Utilities|String|ToString(Integer) _output_get))))

(event Custom|EnablePlayerInput
  (Input|EnableInput (Game|GetPlayerController 0)))

(event Custom|DisablePlayerInput
  (Input|DisableInput (Game|GetPlayerController 0)))

(event Custom|UnlockCarMovement
  ;[1 1 1] Movement
  (Utilities|FlowControl|Sequence
    (:then_0
      (Utilities|FlowControl|Gate false) ; enters at Open
    )
    (:then_1
      (Utilities|FlowControl|Gate false) ; enters at Open
    )
    (:then_2
      (Utilities|FlowControl|Gate false) ; enters at Open
    )
    (:then_3
      (Utilities|FlowControl|Gate false) ; enters at Open
    )))

(event Custom|LockCarMovement
  ;[1 1 1] Movement
  (Utilities|FlowControl|Sequence
    (:then_0
      (Utilities|FlowControl|Gate false) ; enters at Close
    )
    (:then_1
      (Utilities|FlowControl|Gate false) ; enters at Close
    )
    (:then_2
      (Utilities|FlowControl|Gate false) ; enters at Close
    )
    (:then_3
      (Utilities|FlowControl|Gate false) ; enters at Close
    )))

(event Input|EnhancedActionEvents|EnhancedInputActionEA_Forward
  (params (ActionValue :type Boolean) (ElapsedSeconds :type Float%20%28double-precision%29) (TriggeredSeconds :type Float%20%28double-precision%29) (InputAction :type Input%20Action%20Object%20Reference :default "/Game/CarTest/Input/EA_Forward.EA_Forward"))
  ;[1 1 1] Movement
  (Utilities|FlowControl|Gate false
    (:Exit
      (CallFunction|Accelerate "1.000000,0.000000,0.000000"))))

(event Input|EnhancedActionEvents|EnhancedInputActionEA_Backward
  (params (ActionValue :type Boolean) (ElapsedSeconds :type Float%20%28double-precision%29) (TriggeredSeconds :type Float%20%28double-precision%29) (InputAction :type Input%20Action%20Object%20Reference :default "/Game/CarTest/Input/EA_Backward.EA_Backward"))
  ;[1 1 1] Movement
  (Utilities|FlowControl|Gate false
    (:Exit
      (CallFunction|Accelerate "-1.000000,0.000000,0.000000"))))

(event Input|EnhancedActionEvents|EnhancedInputActionEA_Left
  (params (ActionValue :type Boolean) (ElapsedSeconds :type Float%20%28double-precision%29) (TriggeredSeconds :type Float%20%28double-precision%29) (InputAction :type Input%20Action%20Object%20Reference :default "/Game/CarTest/Input/EA_Left.EA_Left"))
  ;[1 1 1] Movement
  (Utilities|FlowControl|Gate false
    (:Exit
      (CallFunction|Accelerate "0.000000,-1.000000,0.000000"))))

(event Input|EnhancedActionEvents|EnhancedInputActionEA_Right
  (params (ActionValue :type Boolean) (ElapsedSeconds :type Float%20%28double-precision%29) (TriggeredSeconds :type Float%20%28double-precision%29) (InputAction :type Input%20Action%20Object%20Reference :default "/Game/CarTest/Input/EA_Right.EA_Right"))
  ;[1 1 1] Movement
  (Utilities|FlowControl|Gate false
    (:Exit
      (CallFunction|Accelerate "0.000000,1.000000,0.000000"))))

(event Input|EnhancedActionEvents|EnhancedInputActionEA_Shoot
  (params (ActionValue :type Boolean) (ElapsedSeconds :type Float%20%28double-precision%29) (TriggeredSeconds :type Float%20%28double-precision%29) (InputAction :type Input%20Action%20Object%20Reference :default "/Game/CarTest/Input/EA_Shoot.EA_Shoot"))
  (bind _pizzainstantiationpoint (Variables|Default|GetPizzaInstantiationPoint))
  (bind _returnvalue (Transformation|GetWorldTransform _pizzainstantiationpoint))
  (bind _returnvalue_2 (Game|SpawnActorfromClass "/Game/Blueprints/BP_THEPIZZA.BP_THEPIZZA_C" (Math|Transform|MakeTransform (.location _returnvalue) (.rotation _returnvalue) "1.000000,1.000000,1.000000") "Undefined" "MultiplyWithRoot" 0 0))
  (Class|PrimitiveComponent|SetAllPhysicsLinearVelocity (Variables|/Game/Blueprints/BP_THEPIZZA.BP_THEPIZZA_C|GetStaticMesh _returnvalue_2) (* (Math|Vector|GetRightVector (Variables|Default|GetCannon)) 2e+04) false))

(event EventBeginPlay
  ;[1 1 1] Input Context
  (bind _asplayer_controller (Utilities|Casting|CastToPlayerController (Pawn|GetController)))
  (Utilities|IsValid (PlayerController|LocalPlayerSubsystems|GetEnhancedInputLocalPlayerSubsystem _asplayer_controller)
    (:Is%20Valid
      (Input|AddMappingContext (PlayerController|LocalPlayerSubsystems|GetEnhancedInputLocalPlayerSubsystem _asplayer_controller) "/Game/CarTest/Input/Map_Drive.Map_Drive" 0 "(bIgnoreAllPressedKeysUntilRelease=True,bForceImmediately=False,bNotifyUserSettings=False)"))))

(event EventTick
  (params (DeltaSeconds :type Float%20%28single-precision%29))
  (bind _body (Variables|Default|GetBody))
  (bind _groundcheckpoint (Variables|Default|GetGroundCheckPoint))
  (bind _returnvalue (Transformation|GetWorldTransform _groundcheckpoint))
  (bind _returnvalue_2 (Transformation|GetWorldRotation _body))
  (bind (_roll _pitch) (Math|Rotator|BreakRotator _returnvalue_2))
  (Utilities|FlowControl|Sequence
    (:then_0
      ;[1 1 1] Set Current Velocity
      (Variables|Default|SetCurrentSpeed (Math|Vector|VectorLength (Transformation|GetComponentVelocity (Variables|Default|GetBody)))))
    (:then_1
      ;[1 1 1] Ground Check
      (bind _returnvalue_3 (Collision|LineTraceByChannel (.location _returnvalue) (+ (.location _returnvalue) (* -5e+01 (Math|Vector|GetUpVector (.rotation _returnvalue)))) "TraceTypeQuery4" false 0 "None"))
      (if _returnvalue_3
        (CallFunction|UnlockCarMovement)
        (Class|PrimitiveComponent|SetLinearDamping (Variables|Default|GetBody) 3.0)
        (Variables|Default|SetisGrounded true)
        (else
          (CallFunction|LockCarMovement)
          (Physics|AddForce (Variables|Default|GetBody) "0.000000,0.000000,-2000.000000" "None" true)
          (Class|PrimitiveComponent|SetLinearDamping (Variables|Default|GetBody) 0.01)
          (Variables|Default|SetisGrounded false))))
    (:then_2
      ;[1 1 1] Rotate
      (if (and (Variables|Default|GetisGrounded) (> (Math|Vector|VectorLengthXY (Transformation|GetComponentVelocity (Variables|Default|GetBody))) 1e+02))
        (Transformation|SetWorldRotation (Variables|Default|GetBody) (Math|Rotator|MakeRotator _roll _pitch (.yaw (Math|Rotator|Lerp(Rotator) _returnvalue_2 (Math|Conversions|RotationFromXVector (Transformation|GetComponentVelocity _body)) 0.3 true))) false false)))
    (:then_3
      ;[1 1 1] Engine Audio
      (Audio|Parameter|SetFloatParameter (Variables|Default|Getengine_meta) "RPM" (Math|Float|MapRangeUnclamped (Variables|Default|GetCurrentSpeed) 0.0 7e+03 0.0 2.0) :!class /Script/AudioExtensions.AudioParameterControllerInterface))
    (:then_4
      ;[1 1 1] City noise
      (Audio|Parameter|SetFloatParameter (Variables|Default|GetCity_noise) "Fade out" (Math|Float|MapRangeUnclamped (Variables|Default|GetCurrentSpeed) 0.0 7e+03 0.0 2.0) :!class /Script/AudioExtensions.AudioParameterControllerInterface))
    (:then_5
      (Variables|/Script/Engine.SpringArmComponent|SetTargetArmLength (Variables|Default|GetSpringArm) (Math|Float|Lerp 2e+03 6e+03 (Math|Float|Clamp(Float) (/ (Variables|Default|GetCurrentSpeed) (- (Variables|Default|GetTopSpeed) 8e+02))))))))

(fn ConstructionScript)

(fn Accelerate
  (params (Direction :type Vector))
  (if (< (Variables|Default|GetCurrentSpeed) (Variables|Default|GetTopSpeed))
    (Physics|AddForce (Variables|Default|GetBody) (* Direction (Variables|Default|GetAcceleration)) "None" true)))